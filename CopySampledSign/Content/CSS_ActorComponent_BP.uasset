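; Player-character component that captures a sign's prefab data when the build gun samples a recipe.
; One second after BeginPlay, it binds to the owning player's build gun recipe-sampled event.
; On sampling, it stores SignData from the widget sign under player 0's build gun hit, leaving it unchanged for other targets.
; Holding Left Ctrl while sampling clears the stored data instead.
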(event `self.ReceiveBeginPlay`
  (`parent.ReceiveBeginPlay`)
  (`KismetSystemLibrary.Delay` 1.0)
  (bind _asfgcharacter_player (cast `FGCharacterPlayer` (`self.GetOwner`)))
  (add `FGBuildGun.mOnRecipeSampled` (`FGCharacterPlayer.GetBuildGun` _asfgcharacter_player) (delegate `Recipe Sampled`)))

(event `Recipe Sampled`
  (params (newRecipe :type "FGRecipe Class Reference"))
  (`self.On Recipe Sampled`))

(fn `On Recipe Sampled`
  (locals (`Hit Buildable` :type "FGBuildable Object Reference") (`Saved Sign Data` :type "PrefabSignData Structure"))
  (if (`PlayerController.IsInputKeyDown` (`GameplayStatics.GetPlayerController` 0) "LeftControl")
    (set `self.SignData` (struct))
    (else
      (bind _asfgbuildable (cast `FGBuildable` (`.HitActor` (`GameplayStatics.BreakHitResult` (`FGBuildGun.mHitResult` (`FGCharacterPlayer.GetBuildGun` (cast `FGCharacterPlayer` (`GameplayStatics.GetPlayerCharacter` 0) :!pure true)))))))
      (bind _asfgbuildable_widget_sign (cast `FGBuildableWidgetSign` _asfgbuildable))
      (set `self.SignData` (`FGBuildableWidgetSign.GetSignPrefabData` _asfgbuildable_widget_sign)))))