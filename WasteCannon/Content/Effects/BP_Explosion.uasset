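; Explosion effect actor that produces a large impact with a flash of light and a crater decal.
; On BeginPlay it plays the EinschlagGroß impact component and spawns a large downward-projected decal using a dynamic material instance.
; The Effekts timeline then drives the point light's intensity along with the crater material's alpha and temperature, animating flash, crater visibility and heat together.
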(event `self.ReceiveBeginPlay`
  (bind _decalmaterialinstance (`self.DecalMaterialInstance`))
  (`AudioComponent.Play` (`self.Einschlag_Groß`) 0.2)
  (bind _returnvalue (`KismetMaterialLibrary.CreateDynamicMaterialInstance` "/WasteCannon/Effects/Mat_Krater_Decal.Mat_Krater_Decal"))
  (bind _output_get (set `self.DecalMaterialInstance` _returnvalue))
  (`GameplayStatics.SpawnDecalAttached` _output_get (5000.0 5000.0 5000.0) (`self.DefaultSceneRoot`) "None" (.location (`self.GetTransform`)) (struct :`Pitch` -90.0) "KeepWorldPosition")
  (bind (_direction _light_intensity _krater_alpha _krater_heat) (`Timeline|Effekts`)
    (:`Update`
      (`LightComponent.SetIntensity` (`self.PointLight`) (* _light_intensity 100000000.0))
      (`MaterialInstanceDynamic.SetScalarParameterValue` _decalmaterialinstance "Alpha" _krater_alpha)
      (`MaterialInstanceDynamic.SetScalarParameterValue` _decalmaterialinstance "Temperatur" (* _krater_heat 1600.0)))))

(fn `UserConstructionScript`)